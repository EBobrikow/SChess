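; Player pawn that handles mouse clicks for a game with board cells.
; It clears its CustomDepthEnable flag on BeginPlay and forwards left mouse presses to OnMouseClicked, which is defined outside this file.
; A disconnected leftover branch traces WorldDynamic objects under the cursor, prints the hit actor's name and toggles custom depth rendering on a BoardCell's mesh, but never runs.
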(event EventBeginPlay
  (Variables|Default|SetCustomDepthEnable false))

(event Collision|EventActorBeginOverlap
  (params (OtherActor :type Actor%20Object%20Reference)))

(event EventTick
  (params (DeltaSeconds :type Float%20%28single-precision%29)))

(event Input|MouseEvents|LeftMouseButton
  (params (Key :type Key%20Structure :default "None"))
  (:Pressed
    (Class|PlayerDefPawn|OnMouseClicked)))

(fn ConstructionScript)